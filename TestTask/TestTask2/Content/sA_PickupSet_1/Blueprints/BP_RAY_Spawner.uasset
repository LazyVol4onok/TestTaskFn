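; BP_RAY_Spawner is a short-lived effect actor that activates an energy FX on its Energy component, then destroys itself.
; Tick drives a flag-based countdown: when ready, Muzzlefybc assigns and activates EnergyFX and the MuzzleDelay timer restarts.
; Timer expiry re-arms that activation and starts a two-second delay before destruction.
; No projectile is spawned, and the ProjectileDelay branch is disconnected.
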(event `self.ReceiveTick`
  (params (DeltaSeconds :type "Float (single-precision)"))
  (`|ExecutionSequence`
    (:`then_0`
      ;[1 1 1] Timer
      (if (`self.timeactivemuzzle`)
        (set `self.Muzzletimer` (- (`self.Muzzletimer`) DeltaSeconds))
        (if (<= (`self.Muzzletimer`) 0.0)
          (set `self.Muzzleready` true)
          (set `self.timeactivemuzzle` false)
          (`KismetSystemLibrary.Delay` 2.0)
          (`self.K2_DestroyActor`))))
    (:`then_1`
      ;[1 1 1] Spawn
      (if (`self.Muzzleready`)
        (`self.Muzzlefybc`)
        (set `self.Muzzletimer` (`self.MuzzleDelay`))
        (set `self.Muzzleready` false)
        (set `self.timeactivemuzzle` true)))))

(fn `Muzzlefybc`
  (bind _energy (`self.Energy`))
  (`NiagaraComponent.SetAsset` _energy (`self.EnergyFX`))
  (`ActorComponent.SetActive` _energy true false))

(fn `UserConstructionScript`)