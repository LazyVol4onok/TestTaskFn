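; NestStart is a button-triggered spawner that launches an AI character with start, end and stop parameters.
; PressButton plays an explosion sound, spawns an actor at Cube3, then spawns an AIChar at SpawnPoint and stores it as ControlledCharacter.
; It passes its Start, Start2, End and Stop values, with their timings, to that character's AI controller by message.
; The SendAIController function is an empty stub.
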(event `Press Button`
  (bind (_returnvalue_location _returnvalue_rotation) (`KismetMathLibrary.BreakTransform` (`SceneComponent.K2_GetComponentToWorld` (`self.SpawnPoint`))))
  (`GameplayStatics.PlaySound2D` "/Game/StarterContent/Audio/Explosion_Cue.Explosion_Cue" 1.0 1.0 0.0 null null)
  (`|SpawnActorFromClass` "/Game/sA_PickupSet_1/Blueprints/BP_RAY_Spawner.BP_RAY_Spawner_C" (`SceneComponent.K2_GetComponentToWorld` (`self.Cube3`)) "AlwaysSpawn" "OverrideRootScale" null null)
  (bind _returnvalue (`AIBlueprintHelperLibrary.SpawnAIFromClass` (`self.AIChar`) null _returnvalue_location _returnvalue_rotation true null))
  (set `self.Controlled Character` _returnvalue)
  (message `/Game/Blueprint/BI_SendAIController.SendAIController` (`AIBlueprintHelperLibrary.GetAIController` (`self.Controlled Character`)) (`self.Start`) (`self.End`) (`self.EndTIme`) (`self.StartTime`) (`self.Start2`) (`self.Stop`) (`self.StopTime`)))

(event `self.ReceiveBeginPlay`
  (`parent.ReceiveBeginPlay`))

(fn `SendAIController`
  (params (Start :type "/Game/Blueprint/Nest/NestStart Class Reference") (End :type "/Game/Blueprint/Nest/NestEnd Class Reference") (EndTime :type "Float (double-precision)") (StartTime :type "Float (double-precision)") (Start2 :type Boolean) (Stop :type Boolean) (StopTime :type "Float (double-precision)"))
  (return))

(fn `UserConstructionScript`
  (`parent.UserConstructionScript`))